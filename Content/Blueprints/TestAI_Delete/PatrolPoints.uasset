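; Behavior tree task that picks the next patrol destination for an AI_ALSTEST pawn.
; It writes a random navigable point near the pawn's current patrol point to a Blackboard vector key.
; It then increments the pawn's patrol index, resetting it to zero only once it exceeds the array length, and finishes successfully.
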(event `self.ReceiveExecuteAI`
  (params (OwnerController :type "AIController Object Reference") (ControlledPawn :type "Pawn Object Reference"))
  (bind _asai_alstest (cast `/Game/Blueprints/TestAI_Delete/AI_ALSTEST` ControlledPawn))
  (bind _patrolpoints (`/Game/Blueprints/TestAI_Delete/AI_ALSTEST.PAtrolPoints` _asai_alstest))
  (bind _patrollocation (`/Game/Blueprints/TestAI_Delete/AI_ALSTEST.PatrolLocation` _asai_alstest))
  (`BTFunctionLibrary.SetBlackboardValueAsVector` (`self.blackboardLocation`) (`NavigationSystemV1.K2_GetRandomLocationInNavigableRadius` (`Actor.K2_GetActorLocation` (`|GetArrayItem` _patrolpoints _patrollocation)) 100.0 null null))
  (bind _result (`/Engine/EditorBlueprintResources/StandardMacros.IncrementInt` _patrollocation)
    (:`  `
      (if (> _result (`KismetArrayLibrary.Array_Length` _patrolpoints))
        (set `/Game/Blueprints/TestAI_Delete/AI_ALSTEST.PatrolLocation` 0 _asai_alstest))
      (`self.FinishExecute` true))))