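; Placeable weapon spawner that creates a WeaponPickup of the selected WeaponType at its skeletal mesh's transform.
; The construction script shows the matching prototype weapon mesh as a preview, which is hidden at BeginPlay.
; Twenty seconds after each spawn it respawns the pickup if gone, otherwise the check chain ends.
; It also binds Spawn to the first player controller's death event, replacing a missing pickup immediately.
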(event `self.ReceiveBeginPlay`
  (`SceneComponent.SetVisibility` (`self.SkeletalMesh`) false false)
  (`|ExecutionSequence`
    (:`then_0`
      (bind _returnvalue (`|SpawnActorFromClass` "/Game/Blueprints/Weapons/PickUps/WeaponPickup.WeaponPickup_C" (`SceneComponent.K2_GetComponentToWorld` (`self.SkeletalMesh`)) "Undefined" "OverrideRootScale" null (`self.Weapon Type`) false null :!label _label))
      (set `self.Weapon_Spawned` _returnvalue)
      (`KismetSystemLibrary.Delay` 20.0)
      (`/Engine/EditorBlueprintResources/StandardMacros.IsValid` (`self.Weapon_Spawned`) :!label _label_2
        (:`Is Not Valid`
          (goto _label))))
    (:`then_1`
      (bind _asals_player_controller (cast `/Game/AdvancedLocomotionV4/Blueprints/CharacterLogic/ALS_Player_Controller` (`GameplayStatics.GetPlayerController` 0)))
      (add `/Game/AdvancedLocomotionV4/Blueprints/CharacterLogic/ALS_Player_Controller.PlayerDeath` _asals_player_controller (delegate `Spawn`)))))

(event `Spawn`
  (goto _label_2))

(fn `UserConstructionScript`
  (bind _skeletalmesh (`self.SkeletalMesh`))
  (switch `/Game/Blueprints/Weapons/PickUps/AmmoTypes` (`self.Weapon Type`)
    (:`NewEnumerator0`
      (`SkinnedMeshComponent.SetSkinnedAssetAndUpdate` _skeletalmesh "/Game/PrototypeWeap/Prototype_Pistol.Prototype_Pistol" true))
    (:`NewEnumerator1`
      (`SkinnedMeshComponent.SetSkinnedAssetAndUpdate` _skeletalmesh "/Game/PrototypeWeap/Prototype_AssaultRifle.Prototype_AssaultRifle" true))
    (:`NewEnumerator2`
      (`SkinnedMeshComponent.SetSkinnedAssetAndUpdate` _skeletalmesh "/Game/PrototypeWeap/Prototype_Shotgun.Prototype_Shotgun" true))
    (:`NewEnumerator3`
      (`SkinnedMeshComponent.SetSkinnedAssetAndUpdate` _skeletalmesh "/Game/PrototypeWeap/Prototype_RocketLauncher.Prototype_RocketLauncher" true))))