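; Pushable placeable actor that, on interaction, snaps the player to a push spot and starts a push through their Push_Comp.
; Construction adds an arrow per PushTransforms entry and sets the cube mesh from Pushtypes.
; HandleInteraction picks the nearest push transform within PushRange by squared 2D distance, then uses capsule and line traces to check standing room, floor slope and blocking walls.
; Failure reasons print to screen via CheckValid.
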(event `/Game/AdvancedLocomotionV4/Blueprints/Interfaces/interact.oninteracted`
  (params (player :type "Character Object Reference"))
  (`self.handle interaction` player))

(fn `findclosedpushtrans`
  (params (`character location` :type "Vector2D Structure") (pushrange :type "Float (double-precision)"))
  (returns (BestIndex :type Integer))
  (locals (currenttransformindex :type Integer) (`current distance SQR` :type "Float (double-precision)" :default 0.0) (`ClosetDistance SQR` :type "Float (double-precision)") (closettransformindex :type Integer :default -1))
  (for (_array_element _array_index) (`self.PushTransforms`)
    (set `local.currenttransformindex` _array_index)
    (bind _output_get (set `local.current distance SQR` (`KismetMathLibrary.DistanceSquared2D` (`KismetMathLibrary.Conv_VectorToVector2D` (`KismetMathLibrary.TransformLocation` (`self.GetTransform`) (.location _array_element))) (`local.character location`))))
    (if (< _output_get (`KismetMathLibrary.Square` (`local.pushrange`)))
      (if (or (< (`local.current distance SQR`) (`local.ClosetDistance SQR`)) (< (`local.closettransformindex`) 0))
        (set `local.closettransformindex` (`local.currenttransformindex`))
        (set `local.ClosetDistance SQR` (`local.current distance SQR`)))))
  (return (`local.closettransformindex`)))

(fn `handle interaction`
  (params (player :type "Character Object Reference"))
  (locals (pushComp :type "/Game/Blueprints/pushable/push_Comp Object Reference") (characterstartingtrans :type "Transform Structure"))
  (bind _returnvalue (`self.GetComponentByClass` player "/Game/Blueprints/pushable/push_Comp.push_Comp_C"))
  (bind _returnvalue_2 (`GameplayStatics.GetPlayerCharacter` 0))
  (bind _setcharactertrans_location (`KismetMathLibrary.BreakTransform` (`self.setcharactertrans`)))
  (bind _setcharactertrans_location_2 (`KismetMathLibrary.BreakTransform` (`self.setcharactertrans`)))
  (bind _capsulecomponent (`Character.CapsuleComponent` (`local.player`)))
  (`/Engine/EditorBlueprintResources/StandardMacros.IsValid` player
    (:`Is Valid`
      (`/Engine/EditorBlueprintResources/StandardMacros.IsValid` _returnvalue
        (:`Is Valid`
          (set `local.pushComp` _returnvalue)
          (set `local.characterstartingtrans` (`self.GetTransform` _returnvalue_2))
          (bind _bestindex (`self.findclosedpushtrans` (`KismetMathLibrary.Conv_VectorToVector2D` (`self.K2_GetActorLocation` _returnvalue_2)) (`/Game/Blueprints/pushable/push_Comp.PushRange` (`local.pushComp`))))
          (if (>= _bestindex 0)
            (bind _returnvalue_3 (`KismetMathLibrary.ComposeTransforms` (`|GetArrayItem` (`self.PushTransforms`) _bestindex) (`self.GetTransform`)))
            (set `self.setcharactertrans` (`KismetMathLibrary.MakeTransform` (`KismetMathLibrary.MakeVector` (.x (.location _returnvalue_3)) (.y (.location _returnvalue_3)) (+ (.z (.location _returnvalue_3)) (`CapsuleComponent.GetScaledCapsuleHalfHeight` (`Character.CapsuleComponent` (`local.player`))))) (.rotation _returnvalue_3) (.scale _returnvalue_3)))
            (bind _outhit (`KismetSystemLibrary.CapsuleTraceSingle` (+ _setcharactertrans_location_2 (0.0 0.0 10.0)) (- _setcharactertrans_location_2 (0.0 0.0 10.0)) (`CapsuleComponent.GetScaledCapsuleRadius` _capsulecomponent) (`CapsuleComponent.GetScaledCapsuleHalfHeight` _capsulecomponent) "TraceTypeQuery1" false (`|MakeArray` (`local.player`) :!type "Actor Object Reference") "None" true (struct :`R` 1.0 :`A` 1.0) (struct :`G` 1.0 :`A` 1.0) 2.0))
            (bind (_bblockinghit _binitialoverlap _time _distance _location _impactpoint _normal _impactnormal _physmat _hitactor) (`GameplayStatics.BreakHitResult` _outhit))
            (if (not _binitialoverlap)
              (if (not (< (.z _normal) (`CharacterMovementComponent.K2_GetWalkableFloorZ` (`Character.CharacterMovement` (`local.player`)))))
                (`self.checkValid` "The Floor is not walkable"))
              (bind (_outhit_2 _returnvalue_4) (`KismetSystemLibrary.LineTraceSingle` (`self.K2_GetActorLocation`) _setcharactertrans_location "TraceTypeQuery1" false (`|MakeArray` self (`local.player`) :!type "Actor Object Reference") "None" true (struct :`R` 1.0 :`A` 1.0) (struct :`G` 1.0 :`A` 1.0) 2.0))
              (if (not _returnvalue_4)
                (`self.K2_SetActorTransform` (`local.player`) (`self.setcharactertrans`) false false)
                (`/Game/Blueprints/pushable/push_Comp.begin push` (`local.pushComp`) self)
                (else
                  (`self.checkValid` "wall in way")))
              (else
                (`self.checkValid` "no room to stand")))
            (else
              (`self.checkValid` "no push transform found"))))
        (:`Is Not Valid`
          (`self.checkValid` "push comp not valid"))))
    (:`Is Not Valid`
      (`self.checkValid` "character not valid"))))

(fn `UserConstructionScript`
  (for _array_element (`self.PushTransforms`)
    (`AddComponent|NODE_AddArrowComponent-0` :`RelativeTransform` _array_element)
    (switch `/Game/Blueprints/pushable/pushtypes` (`self.pushtypes`)
      (:`NewEnumerator0`
        (`StaticMeshComponent.SetStaticMesh` (`self.Cube`) "/Game/BlockingStarterPack/Props/IndustryPropsPack6/Meshes/SM_WaterTank01.SM_WaterTank01")))))